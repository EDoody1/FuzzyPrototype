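; Player controller for a side-scroller that handles drop-in joining, leaving and pausing for its player.
; On BeginPlay it reads the stock lives from the StoreSettings game instance and sets an initial rank from the game mode's player maximum.
; Enter or gamepad Start resets stats, spawns through SideScrollerGameMode and increments its active-player count, guarded to run once.
; Backspace or gamepad Back requests a despawn, and P opens the pause menu.
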(event `self.ReceiveBeginPlay`
  (bind _asstore_settings (cast `/Game/Doody/FuzzyPrototype/StoreSettings` (`GameplayStatics.GetGameInstance`)))
  (set `self.Full Lives` (`/Game/Doody/FuzzyPrototype/StoreSettings.StockSetting` _asstore_settings))
  (bind _asside_scroller_game_mode (cast `/Game/Doody/Blueprints/SideScrollerGameMode` (`GameplayStatics.GetGameMode`)))
  (set `self.PRank` (+ (`/Game/Doody/Blueprints/SideScrollerGameMode.MaxPlayers` _asside_scroller_game_mode) 1)))

(event `Key|Enter`
  (params (Key :type "Key Structure"))
  (bind _returnvalue (`GameplayStatics.GetGameMode`))
  (:`Pressed`
    (if (not (> (`self.EnterPresses`) 0)) :!label _label
      (set `self.Lives` (`self.Full Lives`))
      (set `self.PScore` 0)
      (set `self.PRank` 0)
      (bind _asside_scroller_game_mode (cast `/Game/Doody/Blueprints/SideScrollerGameMode` _returnvalue))
      (`/Game/Doody/Blueprints/SideScrollerGameMode.SpawnCharacter` _asside_scroller_game_mode self)
      (set `self.EnterPresses` 1)
      (bind _asside_scroller_game_mode_2 (cast `/Game/Doody/Blueprints/SideScrollerGameMode` _returnvalue))
      (bind _output_get (set `/Game/Doody/Blueprints/SideScrollerGameMode.ActivePlayers` (+ (`/Game/Doody/Blueprints/SideScrollerGameMode.ActivePlayers` _asside_scroller_game_mode_2) 1) _asside_scroller_game_mode_2))
      (`KismetSystemLibrary.PrintString` (`KismetStringLibrary.Concat_StrStr` "Active Players = " (`KismetStringLibrary.Conv_IntToString` _output_get))))))

(event `Key|Gamepad_Special_Right`
  (params (Key :type "Key Structure"))
  (:`Pressed`
    (goto _label)))

(event `Key|Gamepad_Special_Left`
  (params (Key :type "Key Structure"))
  (:`Pressed`
    (bind _asside_scroller_game_mode (cast `/Game/Doody/Blueprints/SideScrollerGameMode` (`GameplayStatics.GetGameMode`) :!label _label_2))
    (`/Game/Doody/Blueprints/SideScrollerGameMode.DespawnCharacter` _asside_scroller_game_mode self)))

(event `Key|BackSpace`
  (params (Key :type "Key Structure"))
  (:`Pressed`
    (goto _label_2)))

(event `Key|P`
  (params (Key :type "Key Structure"))
  (:`Pressed`
    (bind _returnvalue (`|CreateWidget` "/Game/Doody/HUD/PauseMenu.PauseMenu_C"))
    (`UserWidget.AddToViewport` _returnvalue 0)
    (`GameplayStatics.SetGamePaused` true)
    (set `PlayerController.bShowMouseCursor` true (`GameplayStatics.GetPlayerController` 0))))

(fn `UserConstructionScript`)