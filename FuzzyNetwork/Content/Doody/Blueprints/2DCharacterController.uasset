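; Player controller for the 2D characters in FuzzyBump, holding each player's lives, score and rank.
; BeginPlay loads lives from the game instance's stock setting, resets score and rank, and increments the game mode's active player count.
; Gamepad Special Left or Backspace asks the game mode to despawn this controller's character, while P opens a test pause menu.
; An unconnected player-creation chain never runs.
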(event `Key|Enter`
  (params (Key :type "Key Structure")))

(event `self.ReceiveBeginPlay`
  (bind _asfuzzy_bump_game_instance (cast `/Game/Doody/FuzzyPrototype/FuzzyBumpGameInstance` (`GameplayStatics.GetGameInstance`)))
  (set `self.Full Lives` (`/Game/Doody/FuzzyPrototype/FuzzyBumpGameInstance.StockSetting` _asfuzzy_bump_game_instance))
  (bind _asfuzzy_bump_game_mode (cast `/Game/Doody/Blueprints/FuzzyBumpGameMode` (`GameplayStatics.GetGameMode`)))
  (set `self.PRank` (+ (`/Game/Doody/Blueprints/FuzzyBumpGameMode.MaxPlayers` _asfuzzy_bump_game_mode) 1))
  (set `self.Lives` (`self.Full Lives`))
  (set `self.PScore` 0)
  (set `self.PRank` 0)
  (set `self.EnterPresses` 1)
  (bind _asfuzzy_bump_game_mode_2 (cast `/Game/Doody/Blueprints/FuzzyBumpGameMode` (`GameplayStatics.GetGameMode`)))
  (bind _output_get (set `/Game/Doody/Blueprints/FuzzyBumpGameMode.ActivePlayers` (+ (`/Game/Doody/Blueprints/FuzzyBumpGameMode.ActivePlayers` _asfuzzy_bump_game_mode_2) 1) _asfuzzy_bump_game_mode_2))
  (`KismetSystemLibrary.PrintString` (`KismetStringLibrary.Concat_StrStr` "Active Players = " (`KismetStringLibrary.Conv_IntToString` _output_get))))

(event `Key|Gamepad_Special_Left`
  (params (Key :type "Key Structure"))
  (:`Pressed`
    (bind _asfuzzy_bump_game_mode (cast `/Game/Doody/Blueprints/FuzzyBumpGameMode` (`GameplayStatics.GetGameMode`) :!label _label))
    (`/Game/Doody/Blueprints/FuzzyBumpGameMode.DespawnCharacter` _asfuzzy_bump_game_mode self)))

(event `Key|BackSpace`
  (params (Key :type "Key Structure"))
  (:`Pressed`
    (goto _label)))

(event `Key|P`
  (params (Key :type "Key Structure"))
  ;[1 1 1] Test Pause Menu
  (:`Pressed`
    (bind _returnvalue (`|CreateWidget` "/Game/Doody/HUD/PauseMenu.PauseMenu_C"))
    (`UserWidget.AddToViewport` _returnvalue 0)
    (`GameplayStatics.SetGamePaused` true)
    (set `PlayerController.bShowMouseCursor` true (`GameplayStatics.GetPlayerController` 0))))

(fn `UserConstructionScript`)