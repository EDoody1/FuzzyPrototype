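; Shared local-multiplayer camera for a side-scroller that keeps all SideScrollerCharacters in view.
; UpdatePlayers caches the character list, and Tick finds the greatest pairwise distance between them to drive a bounded, interpolated spring arm length for zoom.
; The spring arm also eases toward the players' average location in Y and Z, with offsets and clamps, while X stays at the actor's starting value.
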(event `self.ReceiveBeginPlay`
  ;[1 1 1] Begin Play establishes Initial Values
  (set `self.CameraZPosition` (.z (`SceneComponent.K2_GetComponentLocation` (`self.SpringArm`))))
  (set `self.CameraYPosition` (.y (`SceneComponent.K2_GetComponentLocation` (`self.SpringArm`))))
  (set `self.CameraStartPos` (`KismetMathLibrary.Conv_DoubleToVector` (.x (`self.K2_GetActorLocation`))))
  (set `self.CamMaxZAdj` (`self.CameraMaxZ`))
  (set `self.CamMinZAdj` (`self.CameraMinZ`))
  (set `self.CamMaxYAdj` (`self.CameraMaxY`))
  (set `self.CamMinYAdj` (`self.CameraMinY`)))

(event `self.ReceiveTick`
  (params (DeltaSeconds :type "Float (single-precision)"))
  (set `self.Delta` DeltaSeconds)
  (`self.SetLongestDistanceBewteenPlayers`)
  (`self.Camera Zoom`)
  (`self.Set Camera Position`))

(event `UpdatePlayers`
  (bind _outactors (`GameplayStatics.GetAllActorsOfClass` "/Game/Doody/Blueprints/SideScrollerCharacter.SideScrollerCharacter_C"))
  (set `self.PlayerArray` _outactors))

(event `Camera Zoom`
  (bind _springarm (`self.SpringArm`))
  ;[1 1 1] Sets Zoom via the arm length with min and max
  (set `SpringArmComponent.TargetArmLength` (`KismetMathLibrary.FInterpTo` (`SpringArmComponent.TargetArmLength` _springarm) (`KismetMathLibrary.FMax` (`KismetMathLibrary.FMin` (`self.FurthestDistance`) (`self.MinZoom`)) (`self.MaxZoom`)) (`self.Delta`) 1.0) _springarm))

(event `SetLongestDistanceBewteenPlayers`
  (bind _playerarray (`self.PlayerArray`))
  (bind _storemaxdis (`self.StoreMaxDis`))
  (bind _returnvalue (`KismetArrayLibrary.Array_Length` _playerarray))
  ;[1 1 1] Gets and Sets Longest Distance between players
  (set `self.StoreMaxDis` 0.0)
  (if (> _returnvalue 0)
    (for _index (range (+ _returnvalue 1))
      (for _index_2 (range (+ _index 1) (+ _returnvalue 1))
        (set `self.StoreMaxDis` (`KismetMathLibrary.FMax` (`self.GetDistanceTo` (`|GetArrayItem` _playerarray _index) (`|GetArrayItem` _playerarray _index_2)) _storemaxdis)))
      (set `self.FurthestDistance` (`KismetMathLibrary.FMax` _storemaxdis)))))

(event `Set Camera Position`
  (bind _delta (`self.Delta`))
  ;[1 1 1] Sets Camera position with limits based on Average position of players
  (bind _returnvalue (`GameplayStatics.GetActorArrayAverageLocation` (`self.PlayerArray`)))
  (set `self.CameraYPosition` (`KismetMathLibrary.FInterpTo` (`self.CameraYPosition`) (`KismetMathLibrary.FClamp` (- (.y _returnvalue) (`self.YOffset`)) (`self.CamMinYAdj`) (`self.CamMaxYAdj`)) _delta 1.0))
  (set `self.CameraZPosition` (`KismetMathLibrary.FInterpTo` (`self.CameraZPosition`) (`KismetMathLibrary.FClamp` (- (.z _returnvalue) (`self.ZOffset`)) (`self.CameraMinZ`) (`self.CameraMaxZ`)) _delta 1.0))
  (`SceneComponent.K2_SetWorldLocation` (`self.SpringArm`) (`KismetMathLibrary.MakeVector` (.x (`self.CameraStartPos`)) (`self.CameraYPosition`) (`self.CameraZPosition`)) false false))

(fn `UserConstructionScript`)