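; Game mode for Fuzzy Bump local multiplayer matches, running timed or stock rules from GameInstance settings.
; A delayed Tick drives the countdown, ending timed games through the GameInstance, while a 15-second loop spawns random items.
; Deaths deduct a life, play a player-colored effect and possess an interim pawn until the delayed character respawn.
; In stock mode, players without lives are ranked, and the last elimination pauses into the completion screen.
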(event `self.ReceiveTick`
  (params (DeltaSeconds :type "Float (single-precision)"))
  (if (> (`self.ActivePlayers`) 0)
    (`KismetSystemLibrary.Delay` 1.0)
    (set `self.Seconds` (- (`self.Seconds`) 1))
    (if (< (`self.Seconds`) 0)
      (set `self.Minutes` (- (`self.Minutes`) 1))
      (set `self.Seconds` 59)
      (if (<= (`self.Minutes`) -1)
        (set `self.Seconds` 0)
        (set `self.Minutes` 0)
        (if (== (`self.GameType`) 1)
          (bind _asfuzzy_bump_game_instance (cast `/Game/Doody/FuzzyPrototype/FuzzyBumpGameInstance` (`GameplayStatics.GetGameInstance`)))
          (`/Game/Doody/FuzzyPrototype/FuzzyBumpGameInstance.EndGame` _asfuzzy_bump_game_instance))))))

(event `self.ReceiveBeginPlay`
  (`|ExecutionSequence`
    (:`then_0`
      ;[1 1 1] Set Game Settings from menu Makes HUD
      (bind _asfuzzy_bump_game_instance (cast `/Game/Doody/FuzzyPrototype/FuzzyBumpGameInstance` (`GameplayStatics.GetGameInstance`)))
      (set `self.Minutes` (`/Game/Doody/FuzzyPrototype/FuzzyBumpGameInstance.TimeSettingMin` _asfuzzy_bump_game_instance))
      (set `self.Seconds` (`/Game/Doody/FuzzyPrototype/FuzzyBumpGameInstance.TimeSettingSec` _asfuzzy_bump_game_instance))
      (set `self.Stock` (`/Game/Doody/FuzzyPrototype/FuzzyBumpGameInstance.StockSetting` _asfuzzy_bump_game_instance))
      (set `self.GameType` (`/Game/Doody/FuzzyPrototype/FuzzyBumpGameInstance.GameModeSetting` _asfuzzy_bump_game_instance)))
    (:`then_1`
      ;[1 1 1] Get Spawn Points from Level
      (bind _outactors (`GameplayStatics.GetAllActorsOfClass` "/Script/Engine.PlayerStart"))
      (set `self.SpawnPoints` _outactors))
    (:`then_2`
      (`self.Spawn Items`))))

(event `Spawn Items`
  (bind _actorlist (`self.ActorList`))
  ;[1 1 1] SpawnItems
  (`KismetSystemLibrary.Delay` 15.0 :!label _label)
  (if (>= 1 (`KismetArrayLibrary.Array_Length` (`self.ItemDrops`)))
    (`|SpawnActorFromClass` (`|GetArrayItem` _actorlist (`KismetMathLibrary.RandomInteger` (`KismetArrayLibrary.Array_Length` _actorlist))) (`self.GetRandomSpawn`) "DontSpawnIfColliding" "OverrideRootScale" null null)
    (goto _label)))

(event `SpawnCharacter`
  (params (PlayerController :type "PlayerController Object Reference"))
  (bind _returnvalue (`Controller.K2_GetPawn` PlayerController))
  (bind _activeplayers (`self.ActivePlayers`))
  (bind _as2dcharacter_controller (cast `/Game/Doody/Blueprints/2DCharacterController` PlayerController))
  (if (== (`/Game/Doody/Blueprints/2DCharacterController.Lives` _as2dcharacter_controller) 0)
    (bind _asfuzzy_bump_game_instance (cast `/Game/Doody/FuzzyPrototype/FuzzyBumpGameInstance` (`GameplayStatics.GetGameInstance`)))
    (if (== (`/Game/Doody/FuzzyPrototype/FuzzyBumpGameInstance.GameModeSetting` _asfuzzy_bump_game_instance) 0)
      (bind _returnvalue_2 (`GameplayStatics.GetPlayerControllerID` _as2dcharacter_controller))
      (bind _result (`/Engine/EditorBlueprintResources/StandardMacros.IncrementInt` _returnvalue_2)
        (:`  `
          (`KismetSystemLibrary.PrintString` (`KismetStringLibrary.Concat_StrStr` "PLAYER " (`KismetStringLibrary.Conv_IntToString` _result) " ELIMINATED"))
          (bind _result_2 (`/Engine/EditorBlueprintResources/StandardMacros.IncrementInt` (`self.EliminatedPlayers`))
            (:`  `
              (set `self.EliminatedPlayers` _result_2)
              (bind _as2dcharacter_controller_2 (cast `/Game/Doody/Blueprints/2DCharacterController` PlayerController))
              (set `/Game/Doody/Blueprints/2DCharacterController.PRank` (- (`self.ActivePlayers`) (`self.EliminatedPlayers`)) _as2dcharacter_controller_2)
              (if (> (`KismetMathLibrary.Conv_IntToByte` _activeplayers) 1)
                (if (== (`self.EliminatedPlayers`) (- _activeplayers 1))
                  (`KismetSystemLibrary.Delay` 1.0)
                  ;[1 1 1] End Game if its Stock
                  (if (== (`self.GameType`) 0)
                    (bind _returnvalue_3 (`|CreateWidget` "/Game/Doody/HUD/GameCompleteStock.GameCompleteStock_C"))
                    (`UserWidget.AddToViewport` _returnvalue_3 0)
                    (set `PlayerController.bShowMouseCursor` true (`GameplayStatics.GetPlayerController` 0))
                    (`GameplayStatics.SetGamePaused` true))))))))
      (else
        (`/Engine/EditorBlueprintResources/StandardMacros.IsValid` _returnvalue :!label _label_2
          (:`Is Valid`
            (`self.K2_DestroyActor` _returnvalue)
            (bind _returnvalue_4 (`|SpawnActorFromClass` "/Game/Doody/Blueprints/SideScrollerCharacter.SideScrollerCharacter_C" (`self.GetRandomSpawn`) "Undefined" "OverrideRootScale" null 0 "1200.000000,-200.000000,720.000000|0.000000,0.000000,0.000000|1.000000,1.000000,1.000000" null))
            (`Controller.Possess` PlayerController _returnvalue_4)))))
    (else
      (goto _label_2))))

(event `DespawnCharacter`
  (params (PlayerController :type "PlayerController Object Reference"))
  (bind _returnvalue (`Controller.K2_GetPawn` PlayerController))
  (bind _returnvalue_2 (`self.K2_GetActorLocation` _returnvalue))
  (bind _as2dcharacter_controller (cast `/Game/Doody/Blueprints/2DCharacterController` PlayerController))
  (bind _result (`/Engine/EditorBlueprintResources/StandardMacros.DecrementInt` (`/Game/Doody/Blueprints/2DCharacterController.Lives` _as2dcharacter_controller))
    (:`  `
      (bind _output_get (set `/Game/Doody/Blueprints/2DCharacterController.Lives` _result _as2dcharacter_controller))
      (bind _returnvalue_3 (`GameplayStatics.GetPlayerControllerID` _as2dcharacter_controller))
      (bind _result_2 (`/Engine/EditorBlueprintResources/StandardMacros.IncrementInt` _returnvalue_3)
        (:`  `
          (`KismetSystemLibrary.PrintString` (`KismetStringLibrary.Concat_StrStr` "Player " (`KismetTextLibrary.Conv_TextToString` (`KismetTextLibrary.Conv_StringToText` (`KismetStringLibrary.Conv_IntToString` _result_2))) " has " (`KismetStringLibrary.Conv_IntToString` _output_get) " Lives Left"))
          (switch `int` _returnvalue_3
            (:`0`
              (`GameplayStatics.SpawnEmitterAtLocation` "/Game/Doody/FuzzyPrototype/P_HB_GrenadeStorm_Shower_NukeLanding_UpdateRed.P_HB_GrenadeStorm_Shower_NukeLanding_UpdateRed" _returnvalue_2))
            (:`1`
              (`GameplayStatics.SpawnEmitterAtLocation` "/Game/Doody/FuzzyPrototype/P_HB_Grenade_Storm_Shower_NukeLanding_UpdateBlue.P_HB_Grenade_Storm_Shower_NukeLanding_UpdateBlue" _returnvalue_2))
            (:`2`
              (`GameplayStatics.SpawnEmitterAtLocation` "/Game/Doody/FuzzyPrototype/P_HB_GrenadeStorm_Shower_NukeLanding_UpdateGreen.P_HB_GrenadeStorm_Shower_NukeLanding_UpdateGreen" _returnvalue_2))
            (:`3`
              (`GameplayStatics.SpawnEmitterAtLocation` "/Game/Doody/FuzzyPrototype/P_HB_GrenadeStorm_Shower_NukeLanding_UpdateYellow.P_HB_GrenadeStorm_Shower_NukeLanding_UpdateYellow" _returnvalue_2)))
          (`/Engine/EditorBlueprintResources/StandardMacros.IsValid` _returnvalue
            (:`Is Valid`
              (`self.K2_DestroyActor` _returnvalue)
              (bind _returnvalue_4 (`|SpawnActorFromClass` "/Game/Doody/Blueprints/IntPawn.IntPawn_C" (`self.GetRandomSpawn`) "Undefined" "OverrideRootScale" null null))
              (`Controller.Possess` PlayerController _returnvalue_4)
              (if true
                (`KismetSystemLibrary.Delay` (`self.RespawnTime`))
                (bind _as2dcharacter_controller_2 (cast `/Game/Doody/Blueprints/2DCharacterController` PlayerController))
                (bind _asfuzzy_bump_game_mode (cast `/Game/Doody/Blueprints/FuzzyBumpGameMode` (`GameplayStatics.GetGameMode`)))
                (`self.SpawnCharacter` _asfuzzy_bump_game_mode _as2dcharacter_controller_2)))))))))

(fn `Spawn Players`)

(fn `UserConstructionScript`)