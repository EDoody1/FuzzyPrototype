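; CutOutTarget is an actor that publishes its position and size to the PC_Cutoff material parameter collection, apparently to drive a cutout effect in materials.
; The construction script writes Position from the root's world location and Scale from the Sphere's world X scale.
; Tick updates both every frame with the sources swapped: Position from the Sphere, Scale from the root.
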(event `self.ReceiveTick`
  (params (DeltaSeconds :type "Float (single-precision)"))
  (bind _returnvalue_x (`KismetMathLibrary.BreakVector` (`SceneComponent.K2_GetComponentScale` (`self.DefaultSceneRoot`))))
  (`KismetMaterialLibrary.SetScalarParameterValue` "/Game/Doody/FuzzyPrototype/Materials/PC_Cutoff.PC_Cutoff" "Scale" _returnvalue_x)
  (`KismetMaterialLibrary.SetVectorParameterValue` "/Game/Doody/FuzzyPrototype/Materials/PC_Cutoff.PC_Cutoff" "Position" (`KismetMathLibrary.Conv_VectorToLinearColor` (`SceneComponent.K2_GetComponentLocation` (`self.Sphere`)))))

(fn `UserConstructionScript`
  (bind _returnvalue_x (`KismetMathLibrary.BreakVector` (`SceneComponent.K2_GetComponentScale` (`self.Sphere`))))
  (`KismetMaterialLibrary.SetVectorParameterValue` "/Game/Doody/FuzzyPrototype/Materials/PC_Cutoff.PC_Cutoff" "Position" (`KismetMathLibrary.Conv_VectorToLinearColor` (`SceneComponent.K2_GetComponentLocation` (`self.DefaultSceneRoot`))))
  (`KismetMaterialLibrary.SetScalarParameterValue` "/Game/Doody/FuzzyPrototype/Materials/PC_Cutoff.PC_Cutoff" "Scale" _returnvalue_x))