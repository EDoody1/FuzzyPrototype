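; DeathRadius is a shrinking death zone that instantly kills any SideScrollerCharacter leaving its DeathCylinder.
; Tick shrinks the actor's X and Y scale linearly with elapsed time down to a clamped minimum, printing messages at scale milestones.
; It feeds scale and position to the PC_Cutoff material parameter collection, with position also set in the construction script.
; End overlap calls Death on the character, passing player controller 0.
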(event `self.ReceiveTick`
  (params (DeltaSeconds :type "Float (single-precision)"))
  (bind _returnvalue_x (`KismetMathLibrary.BreakVector` (`SceneComponent.K2_GetComponentScale` (`self.DefaultSceneRoot`))))
  (bind _returnvalue (`KismetMathLibrary.FClamp` (- 3.5 (/ (`self.TimePass`) 100.0)) 0.375 3.5))
  (set `self.TimePass` (+ (* DeltaSeconds 1.0) (`self.TimePass`)))
  (`KismetMaterialLibrary.SetScalarParameterValue` "/Game/Doody/FuzzyPrototype/Materials/PC_Cutoff.PC_Cutoff" "Scale" _returnvalue_x)
  (`KismetMaterialLibrary.SetVectorParameterValue` "/Game/Doody/FuzzyPrototype/Materials/PC_Cutoff.PC_Cutoff" "Position" (`KismetMathLibrary.Conv_VectorToLinearColor` (`SceneComponent.K2_GetComponentLocation` (`self.DeathCylinder`))))
  (`self.SetActorScale3D` (`KismetMathLibrary.MakeVector` _returnvalue _returnvalue 1.0))
  (if (`KismetMathLibrary.NearlyEqual_FloatFloat` _returnvalue 3.0 0.0001)
    (`KismetSystemLibrary.PrintText` "Death Scale Now at 3")
    (elif (`KismetMathLibrary.NearlyEqual_FloatFloat` _returnvalue 2.0 0.0001)
      (`KismetSystemLibrary.PrintText` "Death Scale Now at 2")
      (elif (`KismetMathLibrary.NearlyEqual_FloatFloat` _returnvalue 1.0 0.0001)
        (`KismetSystemLibrary.PrintText` "Death Scale Now at 1")
        (elif (== _returnvalue 0.375)
          (if (`self.PrintDeathScale`)
            (`KismetSystemLibrary.PrintText` "Death Scale Now Sallest!")
            (set `self.PrintDeathScale` false)))))))

(event `self.DeathCylinder.OnComponentEndOverlap`
  (params (OverlappedComponent :type "PrimitiveComponent Object Reference") (OtherActor :type "Actor Object Reference") (OtherComp :type "PrimitiveComponent Object Reference") (OtherBodyIndex :type Integer))
  (`KismetSystemLibrary.PrintString` (`KismetStringLibrary.Concat_StrStr` (`KismetSystemLibrary.GetDisplayName` OtherActor) " HAS LEFT THE ZONE"))
  (bind _asside_scroller_character (cast `/Game/Doody/Blueprints/SideScrollerCharacter` OtherActor))
  (`/Game/Doody/Blueprints/SideScrollerCharacter.Death` _asside_scroller_character (`GameplayStatics.GetPlayerController` OtherActor) true))

(fn `UserConstructionScript`
  (`KismetMaterialLibrary.SetVectorParameterValue` "/Game/Doody/FuzzyPrototype/Materials/PC_Cutoff.PC_Cutoff" "Position" (`KismetMathLibrary.Conv_VectorToLinearColor` (`SceneComponent.K2_GetComponentLocation` (`self.DefaultSceneRoot`)))))